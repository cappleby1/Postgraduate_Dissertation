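; Yellow button actor that spawns a single Box and shows an on-screen message when its capsule is first overlapped.
; Any overlap on the capsule triggers it, and the IsThereBox flag blocks repeat triggers.
; The Box appears at a fixed world X offset from the button.
; A YellowButtontext widget is added to the viewport, then hidden after a short delay rather than removed.
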(event OnComponentBeginOverlap(Shape_WideCapsule)
  (params (OverlappedComponent :type Primitive%20Component%20Object%20Reference) (OtherActor :type Actor%20Object%20Reference) (OtherComp :type Primitive%20Component%20Object%20Reference) (OtherBodyIndex :type Integer) (bFromSweep :type Boolean) (SweepResult :type Hit%20Result%20Structure%20%28by%20ref%29))
  (if (not (Variables|Default|GetIsThereBox))
    (Variables|Default|SetIsThereBox true)
    (Game|SpawnActorfromClass "/Game/Blueprints/Actors/Box.Box_C" (Math|Conversions|ToTransform(Vector) (+ (Transformation|GetActorLocation) "70.000000,0.000000,0.000000")) "Undefined" "MultiplyWithRoot" 0 0)
    (bind _returnvalue (UserInterface|CreateWidget "/Game/Blueprints/Menu/YellowButtontext.YellowButtontext_C"))
    (UserInterface|Viewport|AddtoViewport _returnvalue 0)
    (Utilities|FlowControl|Delay 3.0)
    (Widget|SetVisibility _returnvalue "Hidden")))

(event EventBeginPlay)

(event Collision|EventActorBeginOverlap
  (params (OtherActor :type Actor%20Object%20Reference)))

(event EventTick
  (params (DeltaSeconds :type Float%20%28single-precision%29)))

(fn ConstructionScript)